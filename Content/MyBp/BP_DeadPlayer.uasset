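; BP_DeadPlayer is a dead-player pawn that provides mouse look and keyboard movement.
; Turn and LookUp axes drive controller yaw and pitch, scaled by MouseSensitivity and world delta seconds.
; MoveForward and MoveRight add movement input along the full control rotation's forward and right vectors, so the forward direction follows camera pitch as well as yaw.
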(event Input|AxisEvents|InputAxisTurn
  (params (AxisValue :type Float%20%28single-precision%29))
  ;[1 1 1] 마우스
  (Pawn|Input|AddControllerYawInput (* (Utilities|Time|GetWorldDeltaSeconds) AxisValue (Variables|Default|GetMouseSensitivity))))

(event Input|AxisEvents|InputAxisLookUp
  (params (AxisValue :type Float%20%28single-precision%29))
  ;[1 1 1] 마우스
  (Pawn|Input|AddControllerPitchInput (* AxisValue (Utilities|Time|GetWorldDeltaSeconds) (Variables|Default|GetMouseSensitivity))))

(event Input|AxisEvents|InputAxisMoveForward
  (params (AxisValue :type Float%20%28single-precision%29))
  ;[1 1 1] 키보드
  (Pawn|Input|AddMovementInput (Math|Vector|GetForwardVector (Pawn|GetControlRotation :!class /Script/Engine.Pawn)) AxisValue false))

(event Input|AxisEvents|InputAxisMoveRight
  (params (AxisValue :type Float%20%28single-precision%29))
  ;[1 1 1] 키보드
  (Pawn|Input|AddMovementInput (Math|Vector|GetRightVector (Pawn|GetControlRotation :!class /Script/Engine.Pawn)) AxisValue false))

(fn ConstructionScript)