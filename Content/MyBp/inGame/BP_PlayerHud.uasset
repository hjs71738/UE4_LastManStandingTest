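; BP_PlayerHud is a player HUD Blueprint that toggles the options menu on the ShowOptions event.
; It creates UMG_OptionsMenu on first use, passes the event's parameter into its InputShowOptions, and reuses the cached widget afterwards.
; Showing the menu switches to UI-only input with cursor and keyboard focus.
; CollapseWidget hides it and restores game-only input without the cursor.
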(event Custom|ShowOptions
  (params (NewParam :type Key%20Structure :default "None"))
  (bind _returnvalue (Game|GetPlayerController 0))
  (Utilities|IsValid (Variables|Default|GetOptionsWidget)
    (:Is%20Valid
      (if (Widget|IsVisible (Variables|Default|GetOptionsWidget))
        (CallFunction|CollapseWidget (Variables|Default|GetOptionsWidget))
        (else
          (Widget|SetVisibility (Variables|Default|GetOptionsWidget) "Visible")
          (Input|SetInputModeUIOnly _returnvalue (Variables|Default|GetOptionsWidget) "DoNotLock" :!label _label)
          (Variables|/Script/Engine.PlayerController|SetbShowMouseCursor _returnvalue true)
          (Widget|SetKeyboardFocus (Variables|Default|GetOptionsWidget)))))
    (:Is%20Not%20Valid
      (bind _returnvalue_2 (UserInterface|CreateWidget "/Game/MyBp/inGame/UMG_OptionsMenu.UMG_OptionsMenu_C"))
      (bind _output_get (Variables|Default|SetOptionsWidget _returnvalue_2))
      (UserInterface|Viewport|AddtoViewport _returnvalue_2 0)
      (Variables|/Game/MyBp/inGame/UMG_OptionsMenu.UMG_OptionsMenu_C|SetInputShowOptions _output_get NewParam)
      (goto _label))))

(fn ConstructionScript)

(fn CollapseWidget
  (params (NewParam :type UMG%20Options%20Menu%20Object%20Reference))
  (bind _returnvalue (Game|GetPlayerController 0))
  (Utilities|IsValid NewParam
    (:Is%20Valid
      (Widget|SetVisibility NewParam "Collapsed"))
    (:Is%20Not%20Valid
      _))
  (Input|SetInputModeGameOnly _returnvalue)
  (Variables|/Script/Engine.PlayerController|SetbShowMouseCursor _returnvalue false))