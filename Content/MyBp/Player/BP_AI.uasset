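; BP_AI is a character that wanders by itself, while also keeping player-style look and move input handlers.
; Tick runs through a random Delay of up to two seconds, then AIMoveTo sends it to a random reachable point nearby.
; IsMoving is only ever set false.
; The server and multicast run/walk events are empty, and their speed-switching logic is left disconnected, so running has no effect.
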(event Custom|RunOnServer
  ;[1 1 1] 코멘트
  ;;[1 1 1] 달리기 리플리케이션
)

(event Custom|WalkOnMulticast
  ;[1 1 1] 코멘트
  ;;[1 1 1] 달리기 리플리케이션
)

(event Custom|WalkOnServer
  ;[1 1 1] 코멘트
  ;;[1 1 1] 달리기 리플리케이션
)

(event Custom|RunOnMulticast
  ;[1 1 1] 코멘트
  ;;[1 1 1] 달리기 리플리케이션
)

(event EventTick
  (params (DeltaSeconds :type Float%20%28single-precision%29))
  ;[1 1 1] Ai 랜덤 움직ㄱ임
  (Utilities|FlowControl|Delay (Math|Random|RandomFloatinRange 0.0 2.0))
  (Variables|Default|SetIsMoving false)
  (AI|AIMoveTo self (.RandomLocation (AI|Navigation|GetRandomReachablePointinRadius (Transformation|GetActorLocation) 1.2e+03 0 0)) 0 5.0 false
    (:OnSuccess
      _)
    (:OnFail
      _))
  (Variables|Default|SetIsMoving false))

(event Input|ActionEvents|InputActionRun
  (params (Key :type Key%20Structure))
  ;[1 1 1] 코멘트
)

(event Input|ActionEvents|InputActionRun
  (params (Key :type Key%20Structure))
  ;[1 1 1] 코멘트
  ;;[1 1 1] 달리기
)

(event Input|AxisEvents|InputAxisTurn
  (params (AxisValue :type Float%20%28single-precision%29))
  ;[1 1 1] 마우스
  (Pawn|Input|AddControllerYawInput AxisValue))

(event Input|AxisEvents|InputAxisLookUp
  (params (AxisValue :type Float%20%28single-precision%29))
  ;[1 1 1] 마우스
  (Pawn|Input|AddControllerPitchInput AxisValue))

(event Input|AxisEvents|InputAxisMoveForward
  (params (AxisValue :type Float%20%28single-precision%29))
  ;[1 1 1] 움직임
  (Pawn|Input|AddMovementInput (Math|Vector|GetForwardVector (Math|Rotator|MakeRotator 0.0 0.0 (.Yaw (Math|Rotator|BreakRotator (Pawn|GetControlRotation :!class /Script/Engine.Pawn))))) AxisValue false))

(event Input|AxisEvents|InputAxisMoveRight
  (params (AxisValue :type Float%20%28single-precision%29))
  ;[1 1 1] 움직임
  (Pawn|Input|AddMovementInput (Math|Vector|GetRightVector (Math|Rotator|MakeRotator 0.0 0.0 (.Yaw (Math|Rotator|BreakRotator (Pawn|GetControlRotation :!class /Script/Engine.Pawn))))) AxisValue false))

(fn ConstructionScript)