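; Tagger player character that catches other players in what appears to be a tag game, with mouse look and yaw-relative movement.
; The Trace input fires a debug-drawn box trace forward from the capsule and passes the hit actor to Catch.
; Catch casts it to BP_Player and calls UpdatePlayerStatus on that player's GamePlayPC.
; Run and walk replication events are empty stubs, and the sprint speed logic is disconnected.
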(event Custom|RunOnServer
  ;[1 1 1] 달리기 리플리케이션
)

(event Custom|WalkOnMulticast
  ;[1 1 1] 달리기 리플리케이션
)

(event Custom|Catch
  (params (Player :type Actor%20Object%20Reference))
  ;[1 1 1] 플레이어 잡음
  (bind _asbp_player (Utilities|Casting|CastToBP_Player Player))
  (bind _asgame_play_pc (Utilities|Casting|CastToGamePlayPC (Pawn|GetController _asbp_player)))
  (Default|UpdatePlayerStatus _asgame_play_pc))

(event Custom|WalkOnServer
  ;[1 1 1] 달리기 리플리케이션
)

(event Custom|RunOnMulticast
  ;[1 1 1] 달리기 리플리케이션
)

(event Input|ActionEvents|InputActionRun
  (params (Key :type Key%20Structure :default "None")))

(event Input|ActionEvents|InputActionRun
  (params (Key :type Key%20Structure :default "None"))
  ;[1 1 1] 달리기
)

(event Input|ActionEvents|InputActionTrace
  (params (Key :type Key%20Structure :default "None"))
  (bind _capsulecomponent (Variables|Collision|GetCapsuleComponent))
  (bind _returnvalue (Transformation|GetWorldLocation _capsulecomponent))
  ;[1 1 1] 코멘트
  (:Pressed
    (bind _outhit (Collision|BoxTraceByChannel _returnvalue (+ _returnvalue (* (Math|Vector|GetForwardVector (Transformation|GetWorldRotation _capsulecomponent)) 3e+02)) "50.000000,50.000000,50.000000" "0, 0, 0" "TraceTypeQuery1" false 0 "ForDuration"))
    (CallFunction|Catch (.hitactor _outhit))))

(event Input|AxisEvents|InputAxisTurn
  (params (AxisValue :type Float%20%28single-precision%29))
  ;[1 1 1] 마우스
  (Pawn|Input|AddControllerYawInput (* AxisValue (Variables|Default|GetMouseSensitivity) (Utilities|Time|GetWorldDeltaSeconds))))

(event Input|AxisEvents|InputAxisLookUp
  (params (AxisValue :type Float%20%28single-precision%29))
  ;[1 1 1] 마우스
  (Pawn|Input|AddControllerPitchInput (* AxisValue (Variables|Default|GetMouseSensitivity) (Utilities|Time|GetWorldDeltaSeconds))))

(event Input|AxisEvents|InputAxisMoveForward
  (params (AxisValue :type Float%20%28single-precision%29))
  ;[1 1 1] 움직임
  (Pawn|Input|AddMovementInput (Math|Vector|GetForwardVector (Math|Rotator|MakeRotator 0.0 0.0 (.Yaw (Math|Rotator|BreakRotator (Pawn|GetControlRotation :!class /Script/Engine.Pawn))))) AxisValue false))

(event Input|AxisEvents|InputAxisMoveRight
  (params (AxisValue :type Float%20%28single-precision%29))
  ;[1 1 1] 움직임
  (Pawn|Input|AddMovementInput (Math|Vector|GetRightVector (Math|Rotator|MakeRotator 0.0 0.0 (.Yaw (Math|Rotator|BreakRotator (Pawn|GetControlRotation :!class /Script/Engine.Pawn))))) AxisValue false))

(fn ConstructionScript)